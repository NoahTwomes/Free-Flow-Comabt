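; BP_GrappleHook is a projectile actor that flies in a straight line from its spawn point to a Target actor.
; BeginPlay caches start, end and direction, then sets the ProjectileMovement velocity using MeshSpeed.
; Tick compares squared distances from the start against the Target's current location, snapping the hook to the cached end point and zeroing velocity once reached.
; DistanceToTarget returns the remaining distance to that end point.
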(event `self.ReceiveBeginPlay`
  (set `self.StartingLoc` (`self.K2_GetActorLocation`))
  (set `self.EndLoc` (`self.K2_GetActorLocation` (`self.Target`)))
  (set `self.Direction` (`KismetMathLibrary.Normal` (- (`self.EndLoc`) (`self.StartingLoc`))))
  (set `MovementComponent.Velocity` (* (`self.Direction`) (`self.MeshSpeed`)) (`self.ProjectileMovement`)))

(event `self.ReceiveTick`
  (params (DeltaSeconds :type "Float (single-precision)"))
  (if (>= (`KismetMathLibrary.Vector_DistanceSquared` (`self.K2_GetActorLocation`) (`self.StartingLoc`)) (`KismetMathLibrary.Vector_DistanceSquared` (`self.K2_GetActorLocation` (`self.Target`)) (`self.StartingLoc`)))
    (`self.K2_SetActorLocation` (+ (`self.StartingLoc`) (* (`self.Direction`) (`KismetMathLibrary.Vector_Distance` (`self.StartingLoc`) (`self.EndLoc`)))) false true)
    (set `MovementComponent.Velocity` (0.0 0.0 0.0) (`self.ProjectileMovement`))))

(fn `DistanceToTarget`
  (returns (ReturnValue :type "Float (double-precision)"))
  (return (`KismetMathLibrary.Vector_Distance` (`self.EndLoc`) (`self.K2_GetActorLocation`))))

(fn `UserConstructionScript`)
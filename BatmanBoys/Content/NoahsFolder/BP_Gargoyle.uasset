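; BP_Gargoyle is an actor that toggles the collision of its Sphere component as the player enters and leaves its PlayerCollision volume.
; On player overlap it prints a debug message and disables the Sphere's collision.
; When the player leaves, it waits a short delay, then restores the Sphere to query-only collision.
; A separate Show function sets its Widget component's visibility, with no caller in this Blueprint.
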(event `self.PlayerCollision.OnComponentBeginOverlap`
  (params (OverlappedComponent :type "PrimitiveComponent Object Reference") (OtherActor :type "Actor Object Reference") (OtherComp :type "PrimitiveComponent Object Reference") (OtherBodyIndex :type Integer) (bFromSweep :type Boolean) (SweepResult :type "HitResult Structure (by ref)"))
  (cast `/Game/WorkingCharacter/Player` OtherActor)
  (`KismetSystemLibrary.PrintString` "Is In Sphere")
  (`PrimitiveComponent.SetCollisionEnabled` (`self.Sphere`) "NoCollision"))

(event `self.PlayerCollision.OnComponentEndOverlap`
  (params (OverlappedComponent :type "PrimitiveComponent Object Reference") (OtherActor :type "Actor Object Reference") (OtherComp :type "PrimitiveComponent Object Reference") (OtherBodyIndex :type Integer))
  (cast `/Game/WorkingCharacter/Player` OtherActor)
  (`KismetSystemLibrary.Delay` 3.0)
  (`PrimitiveComponent.SetCollisionEnabled` (`self.Sphere`) "QueryOnly"))

(fn `Show`
  (params (Active :type Boolean))
  (`SceneComponent.SetVisibility` (`self.Widget`) Active false))

(fn `UserConstructionScript`)
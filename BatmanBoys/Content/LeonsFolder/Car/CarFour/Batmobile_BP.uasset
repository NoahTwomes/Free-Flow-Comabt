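; Drivable Batmobile Chaos wheeled vehicle pawn with throttle, brake, steering, handbrake, boost and mouse-orbit camera.
; Boost changes engine torque, toggles Niagara and audio, and nudges FOV one interpolation step per press or release.
; Tick eases spring-arm yaw back to zero, resetting pitch and roll.
; A radius trigger shows an interact prompt; E unhides the Player, moves it to PlayerOutPos and repossesses it.
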(event `self.ReceiveTick`
  (params (DeltaSeconds :type "Float (single-precision)"))
  (`|ExecutionSequence`
    (:`then_0`
      (`PrimitiveComponent.SetAngularDamping` (`self.Mesh`) (`KismetMathLibrary.SelectFloat` 3.0 3.0 (`NavMovementComponent.IsMovingOnGround` (`self.MovementComp`)))) ; Damps rotation when in air
      (`self.InterpsToOriginalRotation`))))

(event `Key|E`
  (params (Key :type "Key Structure"))
  (bind (_returnvalue_location _returnvalue_rotation) (`KismetMathLibrary.BreakTransform` (`SceneComponent.K2_GetComponentToWorld` (`self.Player Out Pos`))))
  (:`Pressed`
    (set `self.isInVehicle` false)
    (bind _returnvalue (`GameplayStatics.GetActorOfClass` "/Game/WorkingCharacter/Player.Player_C"))
    (`self.SetActorHiddenInGame` _returnvalue false)
    (`self.K2_SetActorTransform` _returnvalue (`KismetMathLibrary.MakeTransform` _returnvalue_location _returnvalue_rotation) false true)
    (`Controller.Possess` (`GameplayStatics.GetPlayerController` 0) _returnvalue)))

(event `InterpsToOriginalRotation`
  (bind (_relativerotation_roll _relativerotation_pitch _relativerotation_yaw) (`KismetMathLibrary.BreakRotator` (`SceneComponent.RelativeRotation` (`self.SpringArm`))))
  (`SceneComponent.K2_SetRelativeRotation` (`self.SpringArm`) (`KismetMathLibrary.MakeRotator` 0.0 0.0 (`KismetMathLibrary.FInterpTo` _relativerotation_yaw 0.0 (`GameplayStatics.GetWorldDeltaSeconds`) 1.0)) false false) ; Reset camera to original angle
)

(event `self.Radius.OnComponentBeginOverlap`
  (params (OverlappedComponent :type "PrimitiveComponent Object Reference") (OtherActor :type "Actor Object Reference") (OtherComp :type "PrimitiveComponent Object Reference") (OtherBodyIndex :type Integer) (bFromSweep :type Boolean) (SweepResult :type "HitResult Structure (by ref)"))
  (bind _returnvalue (`GameplayStatics.GetPlayerCharacter` 0))
  (bind _interact_prompt (`self.Interact Prompt`))
  (if (== OtherActor _returnvalue)
    (`UserWidget.AddToViewport` _interact_prompt 0)
    (else
      (if (== _returnvalue (stale `self.Radius.OnComponentEndOverlap` OtherActor)) :!label _label
        (`Widget.RemoveFromParent` _interact_prompt)))))

(event `self.ReceiveBeginPlay`
  (bind _aschaos_wheeled_vehicle_movement_component (cast `ChaosWheeledVehicleMovementComponent` (`self.VehicleMovementComponent`)))
  (set `self.MovementComp` _aschaos_wheeled_vehicle_movement_component)
  (`|ExecutionSequence`
    (:`then_0`
      (bind _returnvalue (`|CreateWidget` "/Game/LeonsFolder/UI/P_Interact.P_Interact_C"))
      (set `self.Interact Prompt` _returnvalue))
    (:`then_1`
      (bind _returnvalue_2 (`|CreateWidget` "/Game/LeonsFolder/UI/W_VehicleUI.W_VehicleUI_C"))
      (`UserWidget.AddToViewport` _returnvalue_2 0))))

(event `InputAxisKey|MouseX`
  (params (AxisValue :type "Float (single-precision)"))
  ;[1 1 1] Camera
  (`SceneComponent.K2_AddRelativeRotation` (`self.SpringArm`) (`KismetMathLibrary.MakeRotator` 0.0 0.0 AxisValue) false false))

(event `self.Radius.OnComponentEndOverlap`
  (params (OverlappedComponent :type "PrimitiveComponent Object Reference") (OtherActor :type "Actor Object Reference") (OtherComp :type "PrimitiveComponent Object Reference") (OtherBodyIndex :type Integer))
  (goto _label))

(event `InputAxisKey|MouseY`
  (params (AxisValue :type "Float (single-precision)"))
  ;[1 1 1] Camera
  (`SceneComponent.K2_AddRelativeRotation` (`self.SpringArm`) (`KismetMathLibrary.MakeRotator` 0.0 AxisValue) false false))

(event `InputAxis|Throttle`
  (params (AxisValue :type "Float (single-precision)"))
  ;[1 1 1] Driving
  (`ChaosVehicleMovementComponent.SetThrottleInput` (`self.VehicleMovementComponent`) AxisValue))

(event `InputAxis|Brake`
  (params (AxisValue :type "Float (single-precision)"))
  ;[1 1 1] Driving
  (`ChaosVehicleMovementComponent.SetBrakeInput` (`self.VehicleMovementComponent`) AxisValue))

(event `InputAxis|Steering`
  (params (AxisValue :type "Float (single-precision)"))
  ;[1 1 1] Driving
  (`ChaosVehicleMovementComponent.SetSteeringInput` (`self.VehicleMovementComponent`) AxisValue))

(event `InputAction|Handbrake`
  (params (Key :type "Key Structure"))
  (bind _vehiclemovementcomponent (`self.VehicleMovementComponent`))
  ;[1 1 1] Driving
  (:`Pressed`
    (`ChaosVehicleMovementComponent.SetHandbrakeInput` _vehiclemovementcomponent true))
  (:`Released`
    (`ChaosVehicleMovementComponent.SetHandbrakeInput` _vehiclemovementcomponent false)))

(event `InputAction|Boost`
  (params (Key :type "Key Structure"))
  (bind _movementcomp (`self.MovementComp`))
  (bind _niagara (`self.Niagara`))
  (bind _camera (`self.Camera`))
  ;[1 1 1] Boost
  (:`Pressed`
    (`CameraComponent.SetFieldOfView` _camera (`KismetMathLibrary.FInterpTo` (`CameraComponent.FieldOfView` (`self.Camera`)) (`self.BoostFOV`) (`GameplayStatics.GetWorldDeltaSeconds`) 5.0))
    (`ChaosWheeledVehicleMovementComponent.SetMaxEngineTorque` _movementcomp 2000.0)
    (`ActorComponent.Activate` _niagara false)
    (`ActorComponent.Activate` (`self.Audio`) false))
  (:`Released`
    (`CameraComponent.SetFieldOfView` _camera (`KismetMathLibrary.FInterpTo` (`CameraComponent.FieldOfView` (`self.Camera`)) (`self.DriveFOV`) (`GameplayStatics.GetWorldDeltaSeconds`) 5.0))
    (`ChaosWheeledVehicleMovementComponent.SetMaxEngineTorque` _movementcomp 750.0)
    (`ActorComponent.Deactivate` _niagara)
    (`ActorComponent.Deactivate` (`self.Audio`))))

(fn `UserConstructionScript`)
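; Grate and vent actor that lets the player enter and exit a vent.
; Enter and exit trigger volumes pass vent availability, actor and target location to the Player, with the exit location raised by capsule half-height.
; Open/CloseVent picks an enter or exit timeline from the player's InVent flag to pitch the Scene component.
; Mesh collision is off during the swing; on finish it returns and InVent flips.
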(event `self.EnterCollision.OnComponentBeginOverlap`
  (params (OverlappedComponent :type "PrimitiveComponent Object Reference") (OtherActor :type "Actor Object Reference") (OtherComp :type "PrimitiveComponent Object Reference") (OtherBodyIndex :type Integer) (bFromSweep :type Boolean) (SweepResult :type "HitResult Structure (by ref)"))
  (if (== OtherActor (`GameplayStatics.GetPlayerCharacter` 0))
    (bind _asplayer (cast `/Game/WorkingCharacter/Player` OtherActor))
    (`/Game/WorkingCharacter/Player.SetVentInfo` _asplayer true self (`SceneComponent.K2_GetComponentLocation` (`self.StaticMesh`)))))

(event `self.EnterCollision.OnComponentEndOverlap`
  (params (OverlappedComponent :type "PrimitiveComponent Object Reference") (OtherActor :type "Actor Object Reference") (OtherComp :type "PrimitiveComponent Object Reference") (OtherBodyIndex :type Integer))
  (if (== OtherActor (`GameplayStatics.GetPlayerCharacter` 0))
    (bind _asplayer (cast `/Game/WorkingCharacter/Player` OtherActor))
    (`/Game/WorkingCharacter/Player.SetVentInfo` _asplayer false null (0.0 0.0 0.0))))

(event `self.ExitCollision.OnComponentBeginOverlap`
  (params (OverlappedComponent :type "PrimitiveComponent Object Reference") (OtherActor :type "Actor Object Reference") (OtherComp :type "PrimitiveComponent Object Reference") (OtherBodyIndex :type Integer) (bFromSweep :type Boolean) (SweepResult :type "HitResult Structure (by ref)"))
  (if (== OtherActor (`GameplayStatics.GetPlayerCharacter` 0))
    (bind _asplayer (cast `/Game/WorkingCharacter/Player` OtherActor))
    (`/Game/WorkingCharacter/Player.SetVentInfo` _asplayer true self (+ (`SceneComponent.K2_GetComponentLocation` (`self.StaticMesh`)) (`KismetMathLibrary.MakeVector` 0.0 0.0 (`CapsuleComponent.CapsuleHalfHeight` (`Character.CapsuleComponent` _asplayer)))))))

(event `self.ExitCollision.OnComponentEndOverlap`
  (params (OverlappedComponent :type "PrimitiveComponent Object Reference") (OtherActor :type "Actor Object Reference") (OtherComp :type "PrimitiveComponent Object Reference") (OtherBodyIndex :type Integer))
  (if (== OtherActor (`GameplayStatics.GetPlayerCharacter` 0))
    (bind _asplayer (cast `/Game/WorkingCharacter/Player` OtherActor))
    (`/Game/WorkingCharacter/Player.SetVentInfo` _asplayer false null (0.0 0.0 0.0))))

(event `Open/Close Vent`
  (bind _staticmesh (`self.StaticMesh`))
  (bind _staticmesh_2 (`self.StaticMesh`))
  (if (`/Game/WorkingCharacter/Player.InVent?` (cast `/Game/WorkingCharacter/Player` (`GameplayStatics.GetPlayerCharacter` 0) :!pure true))
    (bind (_direction _newtrack_0) (`Timeline|VentExit`)
      (:`Update`
        (`PrimitiveComponent.SetCollisionEnabled` _staticmesh_2 "NoCollision")
        (`SceneComponent.K2_SetRelativeRotation` (`self.Scene`) (`KismetMathLibrary.MakeRotator` 0.0 (`KismetMathLibrary.Lerp` 0.0 90.0 _newtrack_0)) false false))
      (:`Finished`
        (`PrimitiveComponent.SetCollisionEnabled` _staticmesh_2 "QueryAndPhysics")
        (set `/Game/WorkingCharacter/Player.InVent?` false (cast `/Game/WorkingCharacter/Player` (`GameplayStatics.GetPlayerCharacter` 0) :!pure true))))
    (else
      (bind (_direction_2 _newtrack_0_2) (`Timeline|VentEnter`)
        (:`Update`
          (`PrimitiveComponent.SetCollisionEnabled` _staticmesh "NoCollision")
          (`SceneComponent.K2_SetRelativeRotation` (`self.Scene`) (`KismetMathLibrary.MakeRotator` 0.0 (`KismetMathLibrary.Lerp` 0.0 90.0 _newtrack_0_2)) false false))
        (:`Finished`
          (`PrimitiveComponent.SetCollisionEnabled` _staticmesh "QueryAndPhysics")
          (set `/Game/WorkingCharacter/Player.InVent?` true (cast `/Game/WorkingCharacter/Player` (`GameplayStatics.GetPlayerCharacter` 0) :!pure true)))))))

(fn `UserConstructionScript`)
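; MovingCaveWall_BP is a cave wall level mechanic that sets up its movement when the player enters its trigger box.
; On Player overlap, it adds two relative control points to InterpToMovement, the origin and MoveToPos, to define the travel path.
; Nothing guards against repeat overlaps, so each one appends the pair again.
; A Batmobile_BP cast and a construction-script copy of the path setup are left unconnected.
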(event `self.Box.OnComponentBeginOverlap`
  (params (OverlappedComponent :type "PrimitiveComponent Object Reference") (OtherActor :type "Actor Object Reference") (OtherComp :type "PrimitiveComponent Object Reference") (OtherBodyIndex :type Integer) (bFromSweep :type Boolean) (SweepResult :type "HitResult Structure (by ref)"))
  (cast `/Game/WorkingCharacter/Player` OtherActor)
  (`InterpToMovementComponent.AddControlPointPosition` (`self.InterpToMovement`) (0.0 0.0 0.0) true)
  (`InterpToMovementComponent.AddControlPointPosition` (`self.InterpToMovement`) (`self.moveToPos`) true))

(fn `UserConstructionScript`)
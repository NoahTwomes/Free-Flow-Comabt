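; BP_Menu3D is a 3D menu actor that hosts a widget and transitions the player's view to other linked menu actors.
; On BeginPlay it binds to the transition event of its BaseMenuClass widget and disables its own collision.
; A valid index from that event selects a LinkedMenus entry, then collision moves from this actor to the target.
; The player controller smoothly blends its view target to the new menu with ease-in-out.
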(event `self.ReceiveBeginPlay`
  (bind _asbase_menu_class (cast `/Game/LeonsFolder/Menus/3D_Main_Menu/Widgets/BaseMenuClass` (`WidgetComponent.GetUserWidgetObject` (`self.Widget`))))
  (add `/Game/LeonsFolder/Menus/3D_Main_Menu/Widgets/BaseMenuClass.TransistionToLinkedMenu` _asbase_menu_class (delegate `TransistionToLinkedMenu_Event`))
  (`self.SetActorEnableCollision` false))

(event `TransistionToLinkedMenu_Event`
  (params (MenuIndex :type Integer))
  (if (`KismetArrayLibrary.Array_IsValidIndex` (`self.LinkedMenus`) MenuIndex)
    (`self.TransistionTo` (`|GetArrayItem` (`self.LinkedMenus`) MenuIndex))))

(event `TransistionTo`
  (params (NewMenu :type "/Game/LeonsFolder/Menus/3D_Main_Menu/BP_Menu3D Object Reference"))
  (`self.SetActorEnableCollision` false)
  (`self.SetActorEnableCollision` NewMenu true)
  (`PlayerController.SetViewTargetWithBlend` (`GameplayStatics.GetPlayerController` 0) NewMenu 2.0 "VTBlend_EaseInOut" 2.0 false))

(fn `UserConstructionScript`)